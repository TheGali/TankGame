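; Player-controllable tank Blueprint that passes its mesh components to native setters and handles camera aiming input.
; AimAzimuth yaws the AzimuthGimbal and AimElavation pitches the SpringArm, both in local space.
; The construction script registers the barrel, casts Turret to TankBarrel for the turret reference, then assigns the turret mesh and clears the barrel's.
; BeginPlay re-registers the barrel and assigns its mesh.
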(event `self.ReceiveBeginPlay`
  (`self.SetBarrelReference` (`self.TankBarrel`))
  (`StaticMeshComponent.SetStaticMesh` (`self.TankBarrel`) "/Game/Tank_assets/tank_fbx_Barrel.tank_fbx_Barrel"))

(event `InputAxis|AimAzimuth`
  (params (AxisValue :type "Float (single-precision)"))
  ;[1 1 1] Camera Input Binding
  (`SceneComponent.K2_AddLocalRotation` (`self.Azimuth Gimbal`) (`KismetMathLibrary.MakeRotator` 0.0 0.0 AxisValue) false false))

(event `InputAxis|AimElavation`
  (params (AxisValue :type "Float (single-precision)"))
  ;[1 1 1] Camera Input Binding
  (`SceneComponent.K2_AddLocalRotation` (`self.SpringArm`) (`KismetMathLibrary.MakeRotator` 0.0 AxisValue) false false))

(fn `UserConstructionScript`
  (`self.SetBarrelReference` (`self.TankBarrel`))
  (bind _astank_barrel (cast `TankBarrel` (`self.Turret`)))
  (`self.SetTurretReference` _astank_barrel)
  (`StaticMeshComponent.SetStaticMesh` (`self.Turret`) "/Game/Tank/tank_fbx_Turret.tank_fbx_Turret")
  (`StaticMeshComponent.SetStaticMesh` (`self.TankBarrel`) null))